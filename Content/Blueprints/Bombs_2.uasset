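; Player 2's bomb actor: it counts down, explodes and updates score and game state in DynaGameInstance.
; BeginPlay lengthens two blast capsules by P2RangeBomb, steps material and light through timed stages, makes a one-shot remote check if flagged, then decrements the owner's bomb count.
; CollideDetect destroys overlapping players, breakable walls and tagged actors, adjusting P2Score and ending the game on player hits.
; A blast emitter spawns before the bomb destroys itself.
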(event EventBeginPlay
  (bind _capsule2 (Variables|Default|GetCapsule2))
  (bind _capsule1 (Variables|Default|GetCapsule1))
  (bind _capsule2_2 (Variables|Default|GetCapsule2))
  (bind _sphere (Variables|Default|GetSphere))
  (bind _pointlight (Variables|Default|GetPointLight))
  ;[1 1 1] Set collision half height according to Instance variable
  (bind _asdyna_game_instance (Utilities|Casting|CastToDynaGameInstance (Game|GetGameInstance)))
  (Variables|Default|SetGameInstance _asdyna_game_instance)
  (Components|Capsule|SetCapsuleHalfHeight _capsule1 (+ (Variables|/Script/Engine.CapsuleComponent|GetCapsuleHalfHeight _capsule2_2) (Variables|/Game/Blueprints/DynaGameInstance.DynaGameInstance_C|GetP2RangeBomb (Variables|Default|GetGameInstance))) true)
  (Components|Capsule|SetCapsuleHalfHeight _capsule2_2 (+ (Variables|/Script/Engine.CapsuleComponent|GetCapsuleHalfHeight _capsule1) (Variables|/Game/Blueprints/DynaGameInstance.DynaGameInstance_C|GetP2RangeBomb (Variables|Default|GetGameInstance))) true)
  ;[1 1 1] Setting the bomb color intensity with delay
  (Rendering|Components|Light|SetIntensity _pointlight 2e+04)
  (Rendering|Material|SetMaterial _sphere 0 "/Game/Materials/Bomb_mat_3.Bomb_mat_3")
  (Utilities|FlowControl|Delay 0.74)
  (Rendering|Components|Light|SetIntensity _pointlight 2e+04)
  (Rendering|Material|SetMaterial _sphere 0 "/Game/Materials/Bomb_mat_2.Bomb_mat_2")
  (Utilities|FlowControl|Delay 0.74)
  (Rendering|Components|Light|SetIntensity _pointlight 4e+04)
  (Rendering|Material|SetMaterial _sphere 0 "/Game/Materials/Bomb_mat_1.Bomb_mat_1")
  (Utilities|FlowControl|Delay 0.74)
  ;[1 1 1] Check for remote controlled bomb
  (if (Variables|Default|Getcontrolledbomb)
    (CallFunction|RemoteControlledBomb 0.0))
  ;[1 1 1] Bomb count manage
  (bind _outactors (Actor|GetAllActorsOfClass "/Game/Blueprints/NewBlueprint_2.NewBlueprint_2_C"))
  (for _array_element _outactors
    (Math|Integer|DecrementInt (Variables|/Game/Blueprints/NewBlueprint_2.NewBlueprint_2_C|GetBom _array_element)))
  ;[1 1 1] Check for overlapping collision actor and manipulate score accordingly
  (CallFunction|CollideDetect _capsule2)
  (CallFunction|CollideDetect (Variables|Default|GetCapsule1))
  (Effects|SpawnEmitteratLocation "/Game/ParticleSystem/BombBlast.BombBlast" (Transformation|GetWorldLocation (Variables|Default|GetSphere)))
  (Actor|DestroyActor)
  (Components|DestroyComponent _capsule2))

(event EventTick
  (params (DeltaSeconds :type Float%20%28single-precision%29)))

(fn ConstructionScript)

(fn CollideDetect
  (params (Target :type Primitive%20Component%20Object%20Reference%20%28by%20ref%29))
  (bind _gameinstance (Variables|Default|GetGameInstance))
  ;[1 1 1] Capsule overlapping actor check collision and manipulate score
  ; To-do
  ; 1)Using raycasting instead of collision check
  ; 2)Shift code to game mode
  (bind _output_get (Variables|Default|SetCollide (Collision|GetOverlappingActors Target 0 :!class /Script/Engine.PrimitiveComponent)))
  (for _array_element _output_get
    (if (== (Utilities|GetClass _array_element) "/Game/Blueprints/NewBlueprint_2.NewBlueprint_2_C")
      (CallFunction|CollideNewBlueprint2 _array_element)
      (Variables|/Game/Blueprints/DynaGameInstance.DynaGameInstance_C|SetP1RangeBomb _gameinstance 0.0 :!label _label)
      (Variables|/Game/Blueprints/DynaGameInstance.DynaGameInstance_C|SetP2RangeBomb _gameinstance 0.0)
      (Variables|/Game/Blueprints/DynaGameInstance.DynaGameInstance_C|SetEndGame _gameinstance true)
      (elif (== (Utilities|GetClass _array_element) "/Game/Blueprints/NewBlueprint.NewBlueprint_C")
        (CallFunction|CollideNewBlueprint _array_element)
        (goto _label)
        (elif (== (Utilities|GetClass _array_element) "/Game/Blueprints/BreakableWall.BreakableWall_C")
          (CallFunction|CollideBreakableWall _array_element)
          (elif (Actor|ActorHasTag _array_element "BombDestroy")
            (Actor|DestroyActor _array_element)
            (elif (== (Utilities|GetClass _array_element) "/Game/Blueprints/Bombs.Bombs_C")
              _)))))))

(fn RangeBooster
  (bind _gameinstance (Variables|Default|GetGameInstance))
  ;[1 1 1] range booster to implement increase in collision capsule half height
  (Variables|/Game/Blueprints/DynaGameInstance.DynaGameInstance_C|SetP2RangeBomb _gameinstance (+ (Variables|/Game/Blueprints/DynaGameInstance.DynaGameInstance_C|GetP2RangeBomb _gameinstance) 5e+01))
  (return))

(fn RemoteControlledBomb
  (params (Timer :type Float%20%28single-precision%29))
  ;[1 1 1] Check for each tick if 10 sec if not check for input
  (if (== Timer 1e+01)
    (return)
    (elif (== (Input|AxisValues|GetPlayer2Remote) 1.0)
      (return))))

(fn RemoteController
  (params (Timer :type Float%20%28single-precision%29))
  (Variables|Default|SetTimer Timer)
  (Variables|Default|Setcontrolledbomb true))

(fn CollideBreakableWall
  (params (NewParam :type Actor%20Object%20Reference))
  (bind _gameinstance (Variables|Default|GetGameInstance))
  ;[1 1 1] Check collision actor set score accordingly and destroy actor
  (bind _asbreakable_wall (Utilities|Casting|CastToBreakableWall NewParam))
  (Default|SpawnRate _asbreakable_wall)
  (Variables|/Game/Blueprints/DynaGameInstance.DynaGameInstance_C|SetP2Score _gameinstance (+ (Variables|/Game/Blueprints/DynaGameInstance.DynaGameInstance_C|GetP2Score _gameinstance) 3e+01))
  (Actor|DestroyActor _asbreakable_wall))

(fn CollideNewBlueprint2
  (params (NewParam :type Actor%20Object%20Reference%20%28by%20ref%29))
  (bind _gameinstance (Variables|Default|GetGameInstance))
  ;[1 1 1] Check collision actor set score accordingly and destroy actor
  (bind _asnew_blueprint_2 (Utilities|Casting|CastToNewBlueprint_2 NewParam)
    (:then
      _)
    (:CastFailed
      _))
  (Variables|/Game/Blueprints/DynaGameInstance.DynaGameInstance_C|SetP2Score _gameinstance (- (Variables|/Game/Blueprints/DynaGameInstance.DynaGameInstance_C|GetP2Score _gameinstance) 5e+02))
  (Actor|DestroyActor _asnew_blueprint_2)
  (return))

(fn CollideNewBlueprint
  (params (NewParam :type Actor%20Object%20Reference%20%28by%20ref%29))
  (bind _gameinstance (Variables|Default|GetGameInstance))
  ;[1 1 1] Check collision actor set score accordingly and destroy actor
  (Variables|/Game/Blueprints/DynaGameInstance.DynaGameInstance_C|SetP2Score _gameinstance (+ (Variables|/Game/Blueprints/DynaGameInstance.DynaGameInstance_C|GetP2Score _gameinstance) 2e+02))
  (bind _asnew_blueprint (Utilities|Casting|CastToNewBlueprint NewParam)
    (:then
      _)
    (:CastFailed
      _))
  (Default|DeleteChar _asnew_blueprint)
  (return))