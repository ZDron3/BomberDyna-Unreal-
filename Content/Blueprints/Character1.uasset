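; Player 1 character Blueprint for a bomb-dropping game with range and remote-control boosters.
; Space spawns a bomb beside the mesh along its right vector until the count reaches MaxBombs0, keeping the latest as Bombs for booster calls.
; SetMeshRotation eases the mesh toward four input-driven facings, playing ZombieRun when none applies.
; DeleteChar only hides the mesh; the remote-control check and its timer are unwired.
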(event EventSetMeshRotation
  (params (SetMeshForward :type Float%20%28single-precision%29) (SetMeshLeft :type Float%20%28single-precision%29))
  (bind _skeletalmesh (Variables|Default|GetSkeletalMesh))
  (bind _relativerotation (Variables|/Script/Engine.SceneComponent|GetRelativeRotation _skeletalmesh))
  ;[1 1 1] Mesh rotation of actor according to input
  (if (== SetMeshForward 1.0)
    (Transformation|SetWorldRotation _skeletalmesh (Math|Interpolation|RInterpTo _relativerotation "0,-90.000000, 0" (Utilities|Time|GetWorldDeltaSeconds) 15.0) false false)
    (elif (== SetMeshForward -1.0)
      (Transformation|SetWorldRotation _skeletalmesh (Math|Interpolation|RInterpTo _relativerotation "0,90.000000, 0" (Utilities|Time|GetWorldDeltaSeconds) 15.0) false false)
      (elif (== SetMeshLeft 1.0)
        (Transformation|SetWorldRotation _skeletalmesh (Math|Interpolation|RInterpTo _relativerotation "0,0.000000, 0" (Utilities|Time|GetWorldDeltaSeconds) 15.0) false false)
        (elif (== SetMeshLeft -1.0)
          (Transformation|SetWorldRotation _skeletalmesh (Math|Interpolation|RInterpTo _relativerotation "0,-180.000000, 0" (Utilities|Time|GetWorldDeltaSeconds) 15.0) false false)
          (else
            (Components|Animation|PlayAnimation (Variables|Default|GetSkeletalMesh) "/Game/Custom/Meshes/RunCharacter/ZombieRun.ZombieRun" true)))))))

(event EventTick
  (params (DeltaSeconds :type Float%20%28single-precision%29))
  ;[1 1 1] Remote control check
)

(event Input|KeyboardEvents|SpaceBar
  (params (Key :type Key%20Structure :default "AnyKey"))
  (bind _skeletalmesh (Variables|Default|GetSkeletalMesh))
  (bind _returnvalue (Transformation|GetWorldLocation _skeletalmesh))
  (bind _returnvalue_2 (Transformation|GetWorldRotation _skeletalmesh))
  (bind (_x _y _z) (Math|Vector|BreakVector _returnvalue))
  (bind _returnvalue_3 (Math|Vector|GetRightVector _returnvalue_2))
  (bind (_x_2 _y_2) (Math|Vector|BreakVector _returnvalue_3))
  ;[1 1 1] Bomb Spawn actor for Player 1
  (:Pressed
    (if (!= (Variables|Default|GetBom_0) (Variables|Default|GetMaxBombs_0))
      (bind _returnvalue_4 (Game|SpawnActorfromClass "/Game/Blueprints/Bombs.Bombs_C" (Math|Conversions|ToTransform(Vector) (Math|Vector|MakeVector (+ _x (* _x_2 1.2e+02)) (+ (* _y_2 1.2e+02) _y) (+ _z 0.0))) "Undefined" 0 0 false false))
      (Math|Integer|IncrementInt (Variables|Default|GetBom_0)
        (:%20%20
          (Variables|Default|SetBombs _returnvalue_4))))))

(fn ConstructionScript)

(fn SetRemoteBomb
  (Class|BombsC|RemoteControl (Variables|Default|GetBombs)))

(fn DeleteChar
  ;[1 1 1] Disappear player 1 as the actor cannot be destroy
  ; To-do
  ; 1)Need to handle Player 1 deletion on bomb collision
  (Rendering|SetVisibility (Variables|Default|GetSkeletalMesh) false false))

(fn RangeBooster
  (Default|RangeBooster (Variables|Default|GetBombs)))