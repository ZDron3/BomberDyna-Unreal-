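; RangeBooster is a pickup actor that boosts the range of the bombs belonging to the character that touches it, then destroys itself.
; Its Box overlap compares the other actor's exact class against NewBlueprint and NewBlueprint_2, then calls RangeBooster on that actor's Bombs.
; Both branches cast to NewBlueprint, so the NewBlueprint_2 branch only takes effect if that class derives from NewBlueprint.
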(event OnComponentBeginOverlap(Box)
  (params (OverlappedComponent :type Primitive%20Component%20Object%20Reference) (OtherActor :type Actor%20Object%20Reference) (OtherComp :type Primitive%20Component%20Object%20Reference) (OtherBodyIndex :type Integer) (bFromSweep :type Boolean) (SweepResult :type Hit%20Result%20Structure%20%28by%20ref%29))
  (if (== (Utilities|GetClass OtherActor) "/Game/Blueprints/NewBlueprint.NewBlueprint_C")
    (bind _asnew_blueprint (Utilities|Casting|CastToNewBlueprint OtherActor))
    (Default|RangeBooster (Variables|/Game/Blueprints/NewBlueprint.NewBlueprint_C|GetBombs _asnew_blueprint))
    (Actor|DestroyActor)
    (elif (== (Utilities|GetClass OtherActor) "/Game/Blueprints/NewBlueprint_2.NewBlueprint_2_C")
      (bind _asnew_blueprint_2 (Utilities|Casting|CastToNewBlueprint OtherActor))
      (Default|RangeBooster (Variables|/Game/Blueprints/NewBlueprint.NewBlueprint_C|GetBombs _asnew_blueprint_2))
      (Actor|DestroyActor))))

(fn ConstructionScript)