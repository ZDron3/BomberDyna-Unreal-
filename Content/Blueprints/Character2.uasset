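; Player 2 character for a bomb-placing game, with range and remote-controller boosters.
; SpawnBomb places a Bombs_2 beside the mesh along its right vector until Bom equals MaxBombs, storing the newest for booster calls.
; SetMeshRotation smoothly turns the mesh to four directions from inputs, looping ZombieRun when none match.
; While RemoteController is set, Tick calls SetRemote, which counts ticks, not seconds, forwarding the count to that bomb until past ten.
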(event EventTick
  (params (DeltaSeconds :type Float%20%28single-precision%29))
  (if (Variables|Default|GetRemoteController)
    (CallFunction|SetRemote)))

(fn ConstructionScript)

(fn SpawnBomb
  (bind _skeletalmesh (Variables|Default|GetSkeletalMesh))
  (bind _returnvalue (Transformation|GetWorldLocation _skeletalmesh))
  (bind _returnvalue_2 (Transformation|GetWorldRotation _skeletalmesh))
  (bind (_x _y _z) (Math|Vector|BreakVector _returnvalue))
  (bind _returnvalue_3 (Math|Vector|GetRightVector _returnvalue_2))
  (bind (_x_2 _y_2) (Math|Vector|BreakVector _returnvalue_3))
  ;[1 1 1] Spawn Bomb 2 for Player 2
  (if (!= (Variables|Default|GetBom) (Variables|Default|GetMaxBombs))
    (bind _returnvalue_4 (Game|SpawnActorfromClass "/Game/Blueprints/Bombs_2.Bombs_2_C" (Math|Conversions|ToTransform(Vector) (Math|Vector|MakeVector (+ _x (* _x_2 1.2e+02)) (+ (* _y_2 1.2e+02) _y) (+ _z 0.0))) "Undefined" 0 0 false false))
    (Math|Integer|IncrementInt (Variables|Default|GetBom)
      (:%20%20
        (Variables|Default|SetBombs _returnvalue_4)))))

(fn SetMeshRotation
  (params (SetMeshForward :type Float%20%28single-precision%29%20%28by%20ref%29) (SetMeshLeft :type Float%20%28single-precision%29%20%28by%20ref%29))
  (bind _skeletalmesh (Variables|Default|GetSkeletalMesh))
  (bind _relativerotation (Variables|/Script/Engine.SceneComponent|GetRelativeRotation _skeletalmesh))
  ;[1 1 1] Set the rotation for character based upon inputs
  (if (== SetMeshForward 1.0)
    (Transformation|SetWorldRotation _skeletalmesh (Math|Interpolation|RInterpTo _relativerotation "0,-90.000000, 0" (Utilities|Time|GetWorldDeltaSeconds) 15.0) false false)
    (return)
    (elif (== SetMeshForward -1.0)
      (Transformation|SetWorldRotation _skeletalmesh (Math|Interpolation|RInterpTo _relativerotation "0,90.000000, 0" (Utilities|Time|GetWorldDeltaSeconds) 15.0) false false)
      (return)
      (elif (== SetMeshLeft 1.0)
        (Transformation|SetWorldRotation _skeletalmesh (Math|Interpolation|RInterpTo _relativerotation "0,0.000000, 0" (Utilities|Time|GetWorldDeltaSeconds) 15.0) false false)
        (return)
        (elif (== SetMeshLeft -1.0)
          (Transformation|SetWorldRotation _skeletalmesh (Math|Interpolation|RInterpTo _relativerotation "0,-180.000000, 0" (Utilities|Time|GetWorldDeltaSeconds) 15.0) false false)
          (return)
          (else
            (Components|Animation|PlayAnimation (Variables|Default|GetSkeletalMesh) "/Game/Custom/Meshes/RunCharacter/ZombieRun.ZombieRun" true)))))))

(fn RangeBooster
  (Default|RangeBooster (Variables|Default|GetBombs)))

(fn SetRemote
  ;[1 1 1] Set remote timer to check ten seconds for each tick called in eventplay after remote controller booster is picked up
  (bind _output_get (Variables|Default|SetRemoteTimer (+ (Variables|Default|GetRemoteTimer) 1.0)))
  (if (<= _output_get 1e+01)
    (Default|RemoteController (Variables|Default|GetBombs) (Variables|Default|GetRemoteTimer))
    (else
      (Variables|Default|SetRemoteController false))))