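; BreakableWall is a wall actor that can drop a random power-up pickup, with its event graph left empty.
; SpawnRate runs a cascade of independent random rolls, trying bomb, range and speed boosters, then a remote controller, and may spawn nothing.
; The chosen pickup spawns at the Cube component's world transform, and a comment marks the drop chances as raised for a demo.
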(event EventBeginPlay)

(event Collision|EventActorBeginOverlap
  (params (OtherActor :type Actor%20Object%20Reference)))

(event EventTick
  (params (DeltaSeconds :type Float%20%28single-precision%29)))

(fn ConstructionScript)

(fn SpawnRate
  (bind _cube (Variables|Default|GetCube))
  (bind _returnvalue (Transformation|GetWorldTransform _cube))
  ;[1 1 1] Creating Spawn chance
  ; currently more than 30% for demo
  (if (< (Math|Random|RandomFloatinRange 0.0 1e+02) 15.0)
    (Game|SpawnActorfromClass "/Game/Blueprints/BombBooster.BombBooster_C" _returnvalue "Undefined" 0 0)
    (elif (< (Math|Random|RandomFloatinRange 0.0 1e+02) 25.0)
      (Game|SpawnActorfromClass "/Game/Blueprints/RangeBooster.RangeBooster_C" _returnvalue "Undefined" 0 0)
      (elif (< (Math|Random|RandomFloatinRange 0.0 1e+02) 45.0)
        (Game|SpawnActorfromClass "/Game/Blueprints/SpeedBooster.SpeedBooster_C" _returnvalue "Undefined" 0 0)
        (elif (< (Math|Random|RandomFloatinRange 0.0 1e+02) 7e+01)
          (Game|SpawnActorfromClass "/Game/Blueprints/RemoteController.RemoteController_C" _returnvalue "Undefined" 0 0))))))