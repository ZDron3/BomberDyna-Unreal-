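; ControllerP1 is a controller Blueprint that also handles Player 2 input, so two players share one game.
; Player2Init spawns a ControllerP2 and a second character at a fixed spot, then has that controller possess it.
; Player 2's axis mappings are forwarded from this controller to that character, driving movement relative to control rotation and updating mesh rotation.
; The Enter key makes the second character spawn a bomb.
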(event EventPlayer2Init
  (bind _returnvalue (Math|Transform|MakeTransform "-900.000000,900.000000,230.000000"))
  ;[1 1 1] Making two controllers using one for 2 Player Input in same Game
  (bind _returnvalue_2 (Game|SpawnActorfromClass "/Game/Blueprints/ControllerP2.ControllerP2_C" _returnvalue "Undefined" 0 0))
  (Variables|Default|SetController2 _returnvalue_2)
  (bind _returnvalue_3 (Game|SpawnActorfromClass "/Game/Blueprints/NewBlueprint_2.NewBlueprint_2_C" _returnvalue "Undefined" 0 0 1e+04))
  (Variables|Default|SetCharacter2 _returnvalue_3)
  (Pawn|Possess (Variables|Default|GetController2) (Variables|Default|GetCharacter2)))

(event Input|AxisEvents|InputAxisForward_Backward2
  (params (AxisValue :type Float%20%28single-precision%29))
  (bind _character2 (Variables|Default|GetCharacter2))
  ;[1 1 1] Using Axis mapping to get Player 2 inputs for the Game
  (Pawn|Input|AddMovementInput _character2 (Math|Vector|GetForwardVector (Pawn|GetControlRotation _character2 :!class /Script/Engine.Pawn)) AxisValue false)
  (Default|SetMeshRotation _character2 AxisValue (stale Input|AxisEvents|InputAxisLeft_Right2 AxisValue)))

(event Input|AxisEvents|InputAxisLeft_Right2
  (params (AxisValue :type Float%20%28single-precision%29))
  (bind _character2 (Variables|Default|GetCharacter2))
  ;[1 1 1] Using Axis mapping to get Player 2 inputs for the Game
  (Pawn|Input|AddMovementInput _character2 (Math|Vector|GetRightVector (Pawn|GetControlRotation _character2 :!class /Script/Engine.Pawn)) AxisValue false)
  (Default|SetMeshRotation _character2 (stale Input|AxisEvents|InputAxisForward_Backward2 AxisValue) AxisValue))

(event Input|KeyboardEvents|Enter
  (params (Key :type Key%20Structure :default "AnyKey"))
  ;[1 1 1] Using Axis mapping to get Player 2 inputs for the Game
  (:Pressed
    (Default|SpawnBomb (Variables|Default|GetCharacter2))))

(fn ConstructionScript)