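; Bomberman-style bomb actor that explodes on BeginPlay after a timed light and material countdown, skipped when Controlledbomb is set.
; The blast destroys tagged actors overlapping two capsules, calls SpawnRate on breakable walls, and spawns a particle burst.
; It decrements the Bom counter on NewBlueprint and NewBlueprint_2 actors, repeating the blast for each class.
; RangeBooster lengthens both capsules; RemoteControlledBomb only adjusts tick interval, without delaying detonation.
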(event EventBeginPlay
  (bind _capsule2 (Variables|Default|GetCapsule2))
  (bind _sphere (Variables|Default|GetSphere))
  (bind _pointlight (Variables|Default|GetPointLight))
  (if (Variables|Default|Getcontrolledbomb)
    (CallFunction|RemoteControlledBomb)
    (else
      (Rendering|Components|Light|SetIntensity _pointlight 2e+04)
      (Rendering|Material|SetMaterial _sphere 0 "/Game/Materials/Bomb_mat_3.Bomb_mat_3")
      (Utilities|FlowControl|Delay 0.74)
      (Rendering|Components|Light|SetIntensity _pointlight 2e+04)
      (Rendering|Material|SetMaterial _sphere 0 "/Game/Materials/Bomb_mat_2.Bomb_mat_2")
      (Utilities|FlowControl|Delay 0.74)
      (Rendering|Components|Light|SetIntensity _pointlight 4e+04)
      (Rendering|Material|SetMaterial _sphere 0 "/Game/Materials/Bomb_mat_1.Bomb_mat_1")
      (Utilities|FlowControl|Delay 0.74)))
  (bind _outactors (Actor|GetAllActorsOfClass "/Game/Blueprints/NewBlueprint.NewBlueprint_C"))
  (for _array_element _outactors
    (Math|Integer|DecrementInt (Variables|/Game/Blueprints/NewBlueprint.NewBlueprint_C|GetBom _array_element)))
  (CallFunction|CollideDetect _capsule2)
  (CallFunction|CollideDetect (Variables|Default|GetCapsule1))
  (bind _returnvalue (Effects|SpawnEmitteratLocation "/Game/ParticleSystem/BombBlast.BombBlast" (Transformation|GetWorldLocation (Variables|Default|GetSphere))))
  (Actor|DestroyActor)
  (Components|DestroyComponent _capsule2)
  (bind _outactors_2 (Actor|GetAllActorsOfClass "/Game/Blueprints/NewBlueprint_2.NewBlueprint_2_C"))
  (for _array_element_2 _outactors_2
    (Math|Integer|DecrementInt (Variables|/Game/Blueprints/NewBlueprint_2.NewBlueprint_2_C|GetBom _array_element_2)))
  (CallFunction|CollideDetect (Variables|Default|GetCapsule2))
  (CallFunction|CollideDetect (Variables|Default|GetCapsule1))
  (bind _returnvalue_2 (Effects|SpawnEmitteratLocation "/Game/ParticleSystem/BombBlast.BombBlast" (Transformation|GetWorldLocation (Variables|Default|GetSphere))))
  (Actor|DestroyActor)
  (Components|DestroyComponent _returnvalue_2))

(fn ConstructionScript)

(fn CollideDetect
  (params (Target :type Primitive%20Component%20Object%20Reference%20%28by%20ref%29))
  (bind _output_get (Variables|Default|SetCollide (Collision|GetOverlappingActors Target 0 :!class /Script/Engine.PrimitiveComponent)))
  (for _array_element _output_get
    (if (Actor|ActorHasTag _array_element "BombDestroy")
      (Actor|DestroyActor _array_element)
      (elif (Actor|ActorHasTag _array_element "BreakWall")
        (bind _asbreakable_wall (Utilities|Casting|CastToBreakableWall _array_element))
        (Default|SpawnRate _asbreakable_wall)
        (Actor|DestroyActor _asbreakable_wall)
        (elif (== (Utilities|GetClass _array_element) "Bombs_C")
          _)))))

(fn RangeBooster
  (bind _capsule1 (Variables|Default|GetCapsule1))
  (bind _capsule2 (Variables|Default|GetCapsule2))
  (Components|Capsule|SetCapsuleHalfHeight _capsule1 (* (Components|Capsule|GetUnscaledCapsuleHalfHeight _capsule1) 1.5) true)
  (Components|Capsule|SetCapsuleHalfHeight _capsule2 (* (Components|Capsule|GetUnscaledCapsuleHalfHeight _capsule2) 1.5) true)
  (return))

(fn RemoteControlledBomb
  (if (== (Input|AxisValues|GetPlayer1Remote) 1.0)
    _
    (else
      (Actor|Tick|SetActorTickInterval 1e+01)))
  (return))