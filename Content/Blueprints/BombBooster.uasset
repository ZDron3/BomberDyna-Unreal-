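; BombBooster is a pickup actor that raises an overlapping player character's maximum bomb count, up to a cap of three.
; Its Box overlap event checks the other actor's class and increments MaxBombs0 on Character1 or MaxBombs on Character2.
; A Character1 overlap always destroys the booster, while a Character2 overlap destroys it only when that character is already at the cap.
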(event OnComponentBeginOverlap(Box)
  (params (OverlappedComponent :type Primitive%20Component%20Object%20Reference) (OtherActor :type Actor%20Object%20Reference) (OtherComp :type Primitive%20Component%20Object%20Reference) (OtherBodyIndex :type Integer) (bFromSweep :type Boolean) (SweepResult :type Hit%20Result%20Structure%20%28by%20ref%29))
  ;[1 1 1] Check collision actor and manipulate accordingly
  (if (== (Utilities|GetClass OtherActor) "/Game/Blueprints/Character1.Character1_C")
    (bind _ascharacter_1 (Utilities|Casting|CastToCharacter1 OtherActor))
    (if (< (Variables|/Game/Blueprints/Character1.Character1_C|GetMaxBombs_0 _ascharacter_1) 3)
      (Math|Integer|IncrementInt (Variables|/Game/Blueprints/Character1.Character1_C|GetMaxBombs_0 _ascharacter_1)
        (:%20%20
          _)))
    (Actor|DestroyActor)
    (elif (== (Utilities|GetClass OtherActor) "/Game/Blueprints/Character2.Character2_C")
      (bind _ascharacter_2 (Utilities|Casting|CastToCharacter2 OtherActor))
      (if (< (Variables|/Game/Blueprints/Character2.Character2_C|GetMaxBombs _ascharacter_2) 3)
        (Math|Integer|IncrementInt (Variables|/Game/Blueprints/Character2.Character2_C|GetMaxBombs _ascharacter_2))
        (else
          (Actor|DestroyActor))))))

(fn ConstructionScript)