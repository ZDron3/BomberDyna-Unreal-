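; A shared camera actor that both local players view, keeping itself centred between two characters.
; On BeginPlay it becomes the view target for both controllers and caches the first two Character actors found.
; Each tick it interpolates toward their midpoint and sets a clamped spring arm length from that smoothed position's distance to world origin, not character separation.
; Arm length drives interpolation speed; the computed Distance vector is unused.
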(event EventBeginPlay
  (Game|Player|SetViewTargetwithBlend (Game|GetPlayerController 0) self 0.0 "VTBlend_Linear" 1.0 false)
  (bind _outactors (Actor|GetAllActorsOfClass "/Script/Engine.Character"))
  (for _index (range 0 1)
    (switch int _index
      (:0
        (Variables|Default|Setc1 (Utilities|Array|Get(acopy) _outactors _index)))
      (:1
        (Variables|Default|Setc2 (Utilities|Array|Get(acopy) _outactors _index))))))

(event EventTick
  (params (DeltaSeconds :type Float%20%28single-precision%29))
  (Variables|Default|SetDistance (- (Transformation|GetActorLocation (Variables|Default|Getc1)) (Transformation|GetActorLocation (Variables|Default|Getc2))))
  (CallFunction|CameraDist)
  (bind _output_get (Variables|Default|SetFocus (Math|Interpolation|VInterpTo (Variables|Default|GetOldPos) (Variables|Default|GetNewPos) (Utilities|Time|GetWorldDeltaSeconds) (Variables|Default|Getinterpspeed))))
  (Transformation|SetActorLocation _output_get false false)
  (Variables|Default|SetOldPos (Transformation|GetActorLocation))
  (bind _output_get_2 (Variables|/Script/Engine.SpringArmComponent|SetTargetArmLength (Variables|Default|GetCameraArm) (Math|Float|Clamp(Float) (* (Math|Vector|VectorLength (Math|Interpolation|VInterpTo (Variables|Default|GetOldPos) (Variables|Default|GetNewPos) (Utilities|Time|GetWorldDeltaSeconds) (Variables|Default|Getinterpspeed))) 2.0) 2e+03 5e+03)))
  (Variables|Default|Setinterpspeed (/ _output_get_2 6e+02)))

(fn ConstructionScript)

(fn CameraDist
  (Variables|Default|SetNewPos (/ (+ (Transformation|GetActorLocation (Variables|Default|Getc1)) (Transformation|GetActorLocation (Variables|Default|Getc2))) 2.0)))