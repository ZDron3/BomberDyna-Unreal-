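; A player-controlled Blueprint that moves on the ground plane and drops bombs.
; Every tick, the ForwardBackward2 and LeftRight2 input axes, scaled by CharacterSpeed, feed the CharacterMovement input vector as world X and Y.
; Pressing Enter spawns a bomb above the Cube component until the Bom counter reaches MaxBombs.
; Each spawn increments the counter, which this graph never decrements, and stores the new bomb in Bombs.
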(event EventTick
  (params (DeltaSeconds :type Float%20%28single-precision%29))
  (bind _characterspeed (Variables|Default|GetCharacterSpeed))
  (Class|PawnMovementComponent|AddInputVector (Variables|Character|GetCharacterMovement) (Math|Vector|MakeVector (* (Input|AxisValues|GetForward/Backward2) _characterspeed) (* (Input|AxisValues|GetLeft/Right2) _characterspeed) 0.0) false))

(event Input|KeyboardEvents|Enter
  (params (Key :type Key%20Structure :default "AnyKey"))
  (bind _cube (Variables|Default|GetCube))
  (bind _returnvalue (Transformation|GetWorldLocation _cube))
  (bind (_x _y _z) (Math|Vector|BreakVector _returnvalue))
  (:Pressed
    (if (!= (Variables|Default|GetBom) (Variables|Default|GetMaxBombs))
      (bind _returnvalue_2 (Game|SpawnActorfromClass "/Game/Blueprint/Bombs.Bombs_C" (Math|Conversions|ToTransform(Vector) (Math|Vector|MakeVector _x _y (+ _z 2.5e+02))) "Undefined" 0 0))
      (Math|Integer|IncrementInt (Variables|Default|GetBom)
        (:%20%20
          (Variables|Default|SetBombs _returnvalue_2))))))

(fn ConstructionScript)