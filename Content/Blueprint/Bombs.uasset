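; Timed bomb actor that destroys overlapping NewBlueprint actors and BreakableWalls when it explodes.
; BeginPlay steps through three delayed fuse stages, swapping the sphere's material and brightening the point light on the last.
; It then decrements Bom on every NewBlueprint actor, runs CollideDetect on two capsules as blast areas, and destroys itself.
; CollideDetect calls SpawnRate on each wall before destroying it.
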(event EventBeginPlay
  (Rendering|Components|Light|SetIntensity (Variables|Default|GetPointLight) 2e+04)
  (Rendering|Material|SetMaterial (Variables|Default|GetSphere) 0 "/Game/Materials/Bomb_mat.Bomb_mat")
  (Utilities|FlowControl|Delay 0.8)
  (Rendering|Components|Light|SetIntensity (Variables|Default|GetPointLight) 2e+04)
  (Rendering|Material|SetMaterial (Variables|Default|GetSphere) 0 "/Game/Materials/Bomb_mat_2.Bomb_mat_2")
  (Utilities|FlowControl|Delay 0.8)
  (Rendering|Components|Light|SetIntensity (Variables|Default|GetPointLight) 4e+04)
  (Rendering|Material|SetMaterial (Variables|Default|GetSphere) 0 "/Game/Materials/Bomb_mat_3.Bomb_mat_3")
  (Utilities|FlowControl|Delay 0.8)
  (bind _outactors (Actor|GetAllActorsOfClass "/Game/Blueprint/NewBlueprint.NewBlueprint_C"))
  (for _array_element _outactors
    (Math|Integer|DecrementInt (Variables|/Game/Blueprint/NewBlueprint.NewBlueprint_C|GetBom _array_element)))
  (CallFunction|CollideDetect (Variables|Default|GetCapsule2))
  (CallFunction|CollideDetect (Variables|Default|GetCapsule1))
  (Actor|DestroyActor))

(fn ConstructionScript)

(fn CollideDetect
  (params (Target :type Primitive%20Component%20Object%20Reference))
  (bind _output_get (Variables|Default|SetCollide (Collision|GetOverlappingActors Target 0 :!class /Script/Engine.PrimitiveComponent)))
  (for _array_element _output_get
    (if (== (Utilities|GetClass _array_element) "/Game/Blueprint/NewBlueprint.NewBlueprint_C")
      (Actor|DestroyActor _array_element)
      (elif (== (Utilities|GetClass _array_element) "/Game/Blueprint/BreakableWall.BreakableWall_C")
        (bind _asbreakable_wall (Utilities|Casting|CastToBreakableWall _array_element))
        (Default|SpawnRate _asbreakable_wall)
        (Actor|DestroyActor _array_element)))))