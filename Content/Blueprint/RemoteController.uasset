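; RemoteController is a Blueprint with a Box trigger that switches an overlapping actor to remote-controlled bombs, apparently as a bomb-game power-up.
; On begin overlap it checks the actor's class against NewBlueprint and NewBlueprint_2 in duplicated branches.
; A match has its bomb limit reduced to a single bomb and the Controlledbomb flag set on its Bombs reference.
; The trigger does not destroy or disable itself afterward.
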(event OnComponentBeginOverlap(Box)
  (params (OverlappedComponent :type Primitive%20Component%20Object%20Reference) (OtherActor :type Actor%20Object%20Reference) (OtherComp :type Primitive%20Component%20Object%20Reference) (OtherBodyIndex :type Integer) (bFromSweep :type Boolean) (SweepResult :type Hit%20Result%20Structure%20%28by%20ref%29))
  (if (== (Utilities|GetClass OtherActor) "/Game/Blueprint/NewBlueprint.NewBlueprint_C")
    (bind _asnew_blueprint (Utilities|Casting|CastToNewBlueprint OtherActor))
    (Variables|/Game/Blueprint/NewBlueprint.NewBlueprint_C|SetMaxBombs _asnew_blueprint 1)
    (Variables|/Game/Blueprint/Bombs.Bombs_C|Setcontrolledbomb (Variables|/Game/Blueprint/NewBlueprint.NewBlueprint_C|GetBombs _asnew_blueprint) true)
    (elif (== (Utilities|GetClass OtherActor) "/Game/Blueprints/NewBlueprint_2.NewBlueprint_2_C")
      (bind _asnew_blueprint_2 (Utilities|Casting|CastToNewBlueprint_2 OtherActor))
      (Variables|/Game/Blueprints/NewBlueprint_2.NewBlueprint_2_C|SetMaxBombs _asnew_blueprint_2 1)
      (Variables|/Game/Blueprints/Bombs.Bombs_C|Setcontrolledbomb (Variables|/Game/Blueprints/NewBlueprint_2.NewBlueprint_2_C|GetBombs _asnew_blueprint_2) true))))

(fn ConstructionScript)